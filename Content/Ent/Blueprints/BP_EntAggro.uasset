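; Aggro Blueprint for the Ent that picks which attack to perform from the distance passed into GetAttack.
; Close range favors the stomp over the hand attack through a weighted random roll.
; Mid range mostly picks the hand attack, sometimes a jump, and occasionally reuses the close-range roll.
; The chosen attack name goes to DoAttack, and nothing fires beyond mid range.
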(event `self.GetAttack`
  (params (distance :type "Float (single-precision)"))
  (if (<= distance 250.0)
    (if (`KismetMathLibrary.RandomBoolWithWeight` 0.7) :!label _label
      (`self.DoAttack` "StompAttack")
      (else
        (`self.DoAttack` "HandAttack" :!label _label_2)))
    (elif (<= distance 400.0)
      (if (`KismetMathLibrary.RandomBoolWithWeight` 0.1)
        (goto _label)
        (elif (`KismetMathLibrary.RandomBoolWithWeight` 0.7)
          (goto _label_2)
          (else
            (`self.DoAttack` "JumpAttack")))))))
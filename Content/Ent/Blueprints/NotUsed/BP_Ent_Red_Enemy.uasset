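; BP_Ent_Red_Enemy is a red Ent minion with a timed lifespan, apparently spawned by BP_EntBoss and stored in a NotUsed folder.
; Thirty seconds after BeginPlay it casts its owner to BP_EntBoss, passes a decremented living-minion count to CheckAliveMinions, then destroys itself only if that cast succeeds.
; The construction script makes the leaves mesh follow the main mesh's pose and sets its visibility from a variable.
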(event `self.ReceiveBeginPlay`
  (`KismetSystemLibrary.Delay` 30.0)
  (bind _asbp_ent_boss (cast `/Game/Ent/Blueprints/BP_EntBoss` (`self.GetOwner`)))
  (`/Game/Ent/Blueprints/BP_EntBoss.CheckAliveMinions` _asbp_ent_boss (- (`/Game/Ent/Blueprints/BP_EntBoss.MinionsAlive` _asbp_ent_boss) 1))
  (`self.K2_DestroyActor`))

(fn `UserConstructionScript`
  (`SkinnedMeshComponent.SetLeaderPoseComponent` (`self.SK_Ent_Leaves`) (`self.Mesh`) true false)
  (`SceneComponent.SetVisibility` (`self.SK_Ent_Leaves`) (`self.Leaves Visability`) false))
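; BP_Root is a root enemy that detects the player within a trigger radius and damages them with knockback.
; It links itself to ABP_Root, updates an in-radius flag each Tick, and runs overlap-based hit checks gated by a DoOnce with a short delayed reset.
; The parry branch is hard-wired off, so hits always deal damage.
; Taking damage plays a hit montage and shows a health bar that fades when a timeline finishes.
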(event `self.CheckIfHit`
  ;[1 0.4462 0.9952] Check if hit player
  (if (`PrimitiveComponent.IsOverlappingActor` (`self.Collider`) (`self.PlayerRef`))
    (`/Engine/EditorBlueprintResources/StandardMacros.DoOnce` false :!label _label
      (:`Completed`
        (if (and (`self.CanBeParried`) false) :!pinned true
          (set `RootAnimInstance.IsParried` true (`self.AnimRef`))
          (else
            (message `IDamageRecievers.TakeDamage` (`self.PlayerRef`) (`self.SmallDamageChange` (`self.DamageToDo`)) 0.0 false 10.0 (`self.K2_GetActorLocation`))))
        (`KismetSystemLibrary.Delay` 0.5)
        (goto _label :!via `Reset`)))))

(event `self.ReceiveBeginPlay`
  ;[0.781 0.99 1] Begin play - setup
  (bind _asplayer_character (cast `PlayerCharacter` (`GameplayStatics.GetPlayerPawn` 0)))
  (set `self.PlayerRef` _asplayer_character)
  (bind _asroot_anim_instance (cast `RootAnimInstance` (`SkeletalMeshComponent.GetAnimInstance` (`self.SkeletalMesh`))))
  (bind _output_get (set `self.AnimRef` _asroot_anim_instance))
  (bind _asabp_root (cast `/Game/Blueprints/Roots/ABP_Root` _output_get))
  (set `/Game/Blueprints/Roots/ABP_Root.RootRef` self _asabp_root))

(event `self.Trigger.OnComponentBeginOverlap`
  (params (OverlappedComponent :type "PrimitiveComponent Object Reference") (OtherActor :type "Actor Object Reference") (OtherComp :type "PrimitiveComponent Object Reference") (OtherBodyIndex :type Integer) (bFromSweep :type Boolean) (SweepResult :type "HitResult Structure (by ref)"))
  ;[1 1 1] OverLapping
  (cast `PlayerCharacter` OtherActor)
  (`self.PlayerInRadius`))

(event `self.UpdateHealthBar`
  (params (DamageTaken :type "Float (single-precision)"))
  ;[1 0.4698 0.4698] Update Health
  (`|PlayMontage` (`self.SkeletalMesh`) "/Game/CarnivorousPlant/Animatios/PlantRoot/Montage_Hit.Montage_Hit"
    (:`then`
      (bind _asenemy_health_bar_widget (cast `/Game/UI/EnemyHealthBar_Widget` (`WidgetComponent.GetWidget` (`self.HealthBar`))))
      (`Widget.SetVisibility` _asenemy_health_bar_widget "HitTestInvisible")
      (`/Game/UI/EnemyHealthBar_Widget.UpdateHealthWidget` _asenemy_health_bar_widget (`self.Health`) (`self.MaxHealth`) DamageTaken)
      (`Timeline|Timeline` :`NewTime` 2.0 :!via `PlayFromStart`
        (:`Finished`
          (`/Game/UI/EnemyHealthBar_Widget.Fade` _asenemy_health_bar_widget))))))

(event `self.ReceiveTick`
  (params (DeltaSeconds :type "Float (single-precision)"))
  ;[1 1 1] OverLapping
  (if (`PrimitiveComponent.IsOverlappingActor` (`self.Trigger`) (`self.PlayerRef`))
    (set `self.PlayerIsInRadius` true)
    (else
      (set `self.PlayerIsInRadius` false))))

(fn `UserConstructionScript`)
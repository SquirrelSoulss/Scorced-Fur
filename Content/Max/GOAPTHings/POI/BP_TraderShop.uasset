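; Trader shop point of interest for the GOAP AI that tells merchants when the player is waiting as a customer.
; Sphere begin and end overlaps with the PlayerCharacter toggle a waiting flag.
; Each change is written to the customerWaiting world state of every Merchant in the level, not just a linked one.
; Begin overlap also prints a debug message for any overlapping actor.
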(event `self.Sphere.OnComponentBeginOverlap`
  (params (OverlappedComponent :type "PrimitiveComponent Object Reference") (OtherActor :type "Actor Object Reference") (OtherComp :type "PrimitiveComponent Object Reference") (OtherBodyIndex :type Integer) (bFromSweep :type Boolean) (SweepResult :type "HitResult Structure (by ref)"))
  (`KismetSystemLibrary.PrintString` "Hello")
  (bind _asplayer_character (cast `PlayerCharacter` OtherActor))
  (`/Engine/EditorBlueprintResources/StandardMacros.IsValid` _asplayer_character
    (:`Is Valid`
      (set `self.IsWating` true)
      (bind _outactors (`GameplayStatics.GetAllActorsOfClass` "/Script/SquirrelSouls.Merchant" :!label _label))
      (for _array_element _outactors
        (`Labourer.ChangeWorldState` _array_element "customerWaiting" (`self.IsWating`))))))

(event `self.Sphere.OnComponentEndOverlap`
  (params (OverlappedComponent :type "PrimitiveComponent Object Reference") (OtherActor :type "Actor Object Reference") (OtherComp :type "PrimitiveComponent Object Reference") (OtherBodyIndex :type Integer))
  (bind _asplayer_character (cast `PlayerCharacter` OtherActor))
  (`/Engine/EditorBlueprintResources/StandardMacros.IsValid` _asplayer_character
    (:`Is Valid`
      (set `self.IsWating` false)
      (goto _label))))

(fn `UserConstructionScript`)
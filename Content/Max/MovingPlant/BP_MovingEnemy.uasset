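; Moving plant enemy Blueprint that patrols an area, damages the player and disintegrates on death.
; Patrol points come from random downward traces inside PatrolArea, and a trader shop event switches its state machine to idle.
; A resettable hurtbox gate limits player hits, while damage briefly reveals a health bar widget.
; Death drives a dynamic disintegration material through a timeline, then destroys the actor.
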(event `self.ReceiveBeginPlay`
  (bind _asenemy_health_bar_widget (cast `/Game/UI/EnemyHealthBar_Widget` (`WidgetComponent.GetWidget` (`self.Widget`))))
  (set `self.As Enemy Health Bar Widget` _asenemy_health_bar_widget)
  (bind _returnvalue (`GameplayStatics.GetActorOfClass` "/Game/Max/GOAPTHings/POI/BP_TraderShop.BP_TraderShop_C"))
  (`/Engine/EditorBlueprintResources/StandardMacros.IsValid` _returnvalue
    (:`Is Valid`
      (add `/Game/Max/GOAPTHings/POI/BP_TraderShop.StopAll` _returnvalue (delegate `Stop`)))))

(event `Stop`
  (`StateManagerComponent.SwitchStateByKey` (`self.stateManager`) "idle"))

(event `self.CallGetPatrolPoint`
  (bind _patrolarea (`self.patrolArea`))
  (bind (_returnvalue_x _returnvalue_y _returnvalue_z) (`KismetMathLibrary.BreakVector` (`SceneComponent.K2_GetComponentLocation` _patrolarea)))
  (bind (_origin _boxextent) (`KismetSystemLibrary.GetComponentBounds` (`self.patrolArea`)))
  (bind (_boxextent_x _boxextent_y _boxextent_z) (`KismetMathLibrary.BreakVector` (`BoxComponent.BoxExtent` _patrolarea)))
  (bind _output_get (set `self.randomPoint` (`KismetMathLibrary.RandomPointInBoundingBox` _origin _boxextent)))
  (bind _outhit (`KismetSystemLibrary.LineTraceSingle` (`KismetMathLibrary.MakeVector` (.x _output_get) (.y _output_get) (+ _boxextent_z _returnvalue_z)) (`KismetMathLibrary.MakeVector` (.x _output_get) (.y _output_get) (- _returnvalue_z _boxextent_z)) "TraceTypeQuery1"))
  (`self.GetPatrolPoint` (`.Location` (`GameplayStatics.BreakHitResult` _outhit))))

(event `self.UpdateHealtbar`
  (params (damage :type "Float (single-precision)"))
  (bind _as_enemy_health_bar_widget (`self.As Enemy Health Bar Widget`))
  (`|ExecutionSequence`
    (:`then_0`
      (`Widget.SetVisibility` _as_enemy_health_bar_widget "HitTestInvisible")
      (`/Game/UI/EnemyHealthBar_Widget.UpdateHealthWidget` _as_enemy_health_bar_widget (`self.health`) (`self.maxHealth`) damage))
    (:`then_1`
      (`KismetSystemLibrary.RetriggerableDelay` 10.0)
      (`Widget.SetVisibility` (`WidgetComponent.GetWidget` (`self.Widget`)) "Collapsed"))))

(event `self.HurtBox.OnComponentBeginOverlap`
  (params (OverlappedComponent :type "PrimitiveComponent Object Reference") (OtherActor :type "Actor Object Reference") (OtherComp :type "PrimitiveComponent Object Reference") (OtherBodyIndex :type Integer) (bFromSweep :type Boolean) (SweepResult :type "HitResult Structure (by ref)"))
  (if (`self.shouldDamage`)
    (`/Engine/EditorBlueprintResources/StandardMacros.DoOnce` false :!label _label
      (:`Completed`
        (bind _asbp_player (cast `/Game/Player/BP_Player` OtherActor))
        (message `IDamageRecievers.TakeDamage` _asbp_player 20.0 0.0 false 0.0 (`self.K2_GetActorLocation`))))))

(event `self.ResetHurtBox`
  (goto _label :!via `Reset`))

(event `self.Mortis`
  (bind _returnvalue (`KismetMaterialLibrary.CreateDynamicMaterialInstance` "/Game/Max/Disintegration/MI_Stationary_Disintegrate.MI_Stationary_Disintegrate"))
  (`PrimitiveComponent.SetMaterial` (`self.Mesh`) 0 _returnvalue)
  (bind (_direction _dis _alpha) (`Timeline|Timeline`)
    (:`Update`
      (`MaterialInstanceDynamic.SetScalarParameterValue` _returnvalue "Alpha" _alpha)
      (`MaterialInstanceDynamic.SetScalarParameterValue` _returnvalue "Fade" _dis))
    (:`Finished`
      (`Widget.SetVisibility` (`WidgetComponent.GetWidget` (`self.Widget`)) "Collapsed")
      (`self.K2_DestroyActor`))))

(fn `UserConstructionScript`
  (bind _returnvalue_location (`KismetMathLibrary.BreakTransform` (`self.GetTransform`)))
  (`SceneComponent.K2_SetWorldTransform` (`self.patrolArea`) (`KismetMathLibrary.MakeTransform` _returnvalue_location) false false))
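; Modular trader NPC built from skeletal mesh parts: two bodies, moustache, beard, beard-with-hair and bags.
; The construction script slaves every part to the main Mesh via Master Pose so they share its animation.
; Per-part boolean variables then set each piece's visibility, allowing different looks from one Blueprint.
; The event graph holds only disabled placeholder events, so no gameplay logic is defined here.
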(fn `UserConstructionScript`
  (`SkinnedMeshComponent.SetLeaderPoseComponent` (`self.SK_Moustache`) (`self.Mesh`) true)
  (`SkinnedMeshComponent.SetLeaderPoseComponent` (`self.SK_Trader_Beard`) (`self.Mesh`) true)
  (`SkinnedMeshComponent.SetLeaderPoseComponent` (`self.SK_Trader_Beard_And_Hair`) (`self.Mesh`) true)
  (`SkinnedMeshComponent.SetLeaderPoseComponent` (`self.SK_Trader_Body_1`) (`self.Mesh`) true)
  (`SkinnedMeshComponent.SetLeaderPoseComponent` (`self.SK_Trader_Body_2`) (`self.Mesh`) true)
  (`SkinnedMeshComponent.SetLeaderPoseComponent` (`self.SK_Bags`) (`self.Mesh`) true)
  (`SceneComponent.SetVisibility` (`self.SK_Moustache`) (`self.Moustache_Visibility`) false)
  (`SceneComponent.SetVisibility` (`self.SK_Trader_Body_1`) (`self.Body_1_Visibility`) false)
  (`SceneComponent.SetVisibility` (`self.SK_Trader_Body_2`) (`self.Body_2_Visibility`) false)
  (`SceneComponent.SetVisibility` (`self.SK_Trader_Beard`) (`self.Beard_Visibility`) false)
  (`SceneComponent.SetVisibility` (`self.SK_Trader_Beard_And_Hair`) (`self.Beard_And_Hair_Visibility`) false)
  (`SceneComponent.SetVisibility` (`self.SK_Bags`) (`self.Bags_Visibility`) false))